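; FollowerInterpolator is an actor that turns toward and follows the player character using interpolation.
; Each Tick, it eases its rotation toward the player with RInterpTo.
; Only once its facing is within a small tolerance does it ease its location toward the player with VInterpTo, both sharing one Speed.
; An unconnected "Smoother floating" variant would move and rotate simultaneously.
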(event `self.ReceiveTick`
  (params (DeltaSeconds :type "Float (single-precision)"))
  (bind _returnvalue (`self.K2_GetActorLocation`))
  (bind _returnvalue_2 (`self.K2_GetActorRotation`))
  (bind _returnvalue_3 (`self.K2_GetActorLocation` (`GameplayStatics.GetPlayerCharacter` 0)))
  (bind _returnvalue_4 (`KismetMathLibrary.Conv_VectorToRotator` (`KismetMathLibrary.Normal` (- _returnvalue_3 _returnvalue))))
  (`self.K2_SetActorRotation` (`KismetMathLibrary.RInterpTo` _returnvalue_2 _returnvalue_4 DeltaSeconds (`self.Speed`)))
  (if (== (`KismetMathLibrary.NormalizedDeltaRotator` _returnvalue_2 _returnvalue_4) (struct) :`ErrorTolerance` 0.1)
    (`self.K2_SetActorLocation` (`KismetMathLibrary.VInterpTo` _returnvalue _returnvalue_3 DeltaSeconds (`self.Speed`)))))

(fn `UserConstructionScript`)