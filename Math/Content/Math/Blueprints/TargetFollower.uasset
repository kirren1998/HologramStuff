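; TargetFollower is a math demo actor that tracks the player character with an arrow and a projection point.
; Each tick it normalizes the vector from itself to the player and rotates the Arrow to face along it.
; It moves Projection along that direction to the player distance multiplied by Scaler, placing it at a proportional point on the line to the player.
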(event `self.ReceiveTick`
  (params (DeltaSeconds :type "Float (single-precision)"))
  (bind _returnvalue (`self.K2_GetActorLocation`))
  (bind _returnvalue_2 (`self.K2_GetActorLocation` (`GameplayStatics.GetPlayerCharacter` 0)))
  (bind _returnvalue_3 (`KismetMathLibrary.Normal` (- _returnvalue_2 _returnvalue)))
  (`SceneComponent.K2_SetWorldRotation` (`self.Arrow`) (`KismetMathLibrary.Conv_VectorToRotator` _returnvalue_3) false false)
  (`SceneComponent.K2_SetWorldLocation` (`self.Projection`) (+ (`self.K2_GetActorLocation`) (* _returnvalue_3 (* (`KismetMathLibrary.Vector_Distance` _returnvalue_2 _returnvalue) (`self.Scaler`)))) false false))

(fn `UserConstructionScript`)