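; Cylinder generator Blueprint that builds a cylinder out of static mesh components in its construction script.
; Nested loops stack rings from Height and HeightSteps, placing meshes around each ring from Radius and RadialSteps.
; Each mesh yaws with its angle around the vertical axis and takes ComponentScale.
; Shift rotates each successive ring by a multiple of the radial step, allowing staggered or twisted patterns.
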(fn `UserConstructionScript`
  (bind _returnvalue (/ 360.0 (`KismetMathLibrary.Conv_IntToDouble` (`self.Radial Steps`))))
  (for _index (range (+ (`self.Height Steps`) 1))
    (for _index_2 (range (+ (`self.Radial Steps`) 1))
      (bind _returnvalue_2 (+ (* (* _index (`self.Shift`)) _returnvalue) (* _index_2 _returnvalue)))
      (`AddComponent|NODE_AddStaticMeshComponent-1` :`RelativeTransform` (`KismetMathLibrary.MakeTransform` (`KismetMathLibrary.GreaterGreater_VectorRotator` (`KismetMathLibrary.MakeVector` (`self.Radius`) 0.0 (* _index (/ (`self.Height`) (`KismetMathLibrary.Conv_IntToDouble` (`self.Height Steps`))))) (`KismetMathLibrary.MakeRotator` 0.0 0.0 _returnvalue_2)) (`KismetMathLibrary.MakeRotator` 0.0 0.0 _returnvalue_2) (`self.Component Scale`))))))